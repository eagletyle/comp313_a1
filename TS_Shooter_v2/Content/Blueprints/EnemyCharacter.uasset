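; EnemyCharacter is an enemy that damages MainCharacter on overlap and awards score when killed.
; A looping timer calls DamageMain at AttacksPerSecond while the player overlaps it.
; AffectHealth runs CalculateHealth; on death it ignores world collision channels, increments the TS_Mode score, detaches its controller and is destroyed after a delay.
; The construction script tints the body with EnemyColour through a dynamic material instance.
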(event `/Game/Blueprints/iDamageable.AffectHealth`
  (params (Delta :type "Float (single-precision)"))
  (bind _capsulecomponent (`self.CapsuleComponent`))
  (`self.CalculateHealth` Delta)
  (if (`self.isDead`)
    (`PrimitiveComponent.SetCollisionResponseToChannel` _capsulecomponent "ECC_WorldDynamic" "ECR_Ignore")
    (`PrimitiveComponent.SetCollisionResponseToChannel` _capsulecomponent "ECC_WorldStatic" "ECR_Ignore")
    (bind _asts_mode (cast `/Game/Blueprints/TS_Mode` (`GameplayStatics.GetGameMode`)))
    (`/Game/Blueprints/TS_Mode.Increment Score` _asts_mode (`self.Score`))
    (`self.DetachFromControllerPendingDestroy`)
    (`KismetSystemLibrary.Delay` 3.0)
    (`self.K2_DestroyActor`)))

(event `self.ReceiveActorBeginOverlap`
  (params (OtherActor :type "Actor Object Reference"))
  (bind _asmain_character (cast `/Game/Blueprints/MainCharacter` OtherActor))
  (set `self.Main` _asmain_character)
  (`KismetSystemLibrary.K2_SetTimer` null "DamageMain" (/ 1.0 (`self.AttacksPerSecond`)) true))

(event `self.ReceiveActorEndOverlap`
  (params (OtherActor :type "Actor Object Reference"))
  (if (== OtherActor (`self.Main`))
    (`KismetSystemLibrary.K2_ClearTimer` null "DamageMain")))

(event `DamageMain`
  (`/Game/Blueprints/MainCharacter.AffectHealth` (`self.Main`) (`self.Damage`)))

(fn `UserConstructionScript`
  (bind _returnvalue (`PrimitiveComponent.CreateDynamicMaterialInstance` (`self.Mesh`) 0 null "None"))
  (bind _output_get (set `self.NewMaterial` _returnvalue))
  (`MaterialInstanceDynamic.SetVectorParameterValue` _output_get "BodyColor" (`self.EnemyColour`)))