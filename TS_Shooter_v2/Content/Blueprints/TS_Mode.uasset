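; Game mode that runs enemy spawning, player respawning and score keeping.
; On begin play it starts a looping timer that calls SpawnEnemy on the first EnemySpawner in the level, at a rate set by EnemiesPerSecond.
; Respawning destroys all EnemyCharacters, then spawns a new MainCharacter at the stored transform and has player controller 0 possess it.
; Score changes are calculated through GetIncrementGameScore.
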(event `self.ReceiveBeginPlay`
  (bind _outactors (`GameplayStatics.GetAllActorsOfClass` "/Game/Blueprints/EnemySpawner.EnemySpawner_C"))
  (bind _output_get (set `self.Spawner` (`|GetArrayItem` _outactors)))
  (`KismetSystemLibrary.K2_SetTimer` _output_get "SpawnEnemy" (/ 1.0 (`self.EnemiesPerSecond`)) true))

(event `Respawn Player`
  (bind _outactors (`GameplayStatics.GetAllActorsOfClass` "/Game/Blueprints/EnemyCharacter.EnemyCharacter_C"))
  (for _array_element _outactors
    (`self.K2_DestroyActor` _array_element))
  (bind _returnvalue (`|SpawnActorFromClass` "/Game/Blueprints/MainCharacter.MainCharacter_C" (`self.Player Spawn Transform`) "Undefined" "OverrideRootScale" null null))
  (`Controller.Possess` (`GameplayStatics.GetPlayerController` 0) _returnvalue))

(event `Increment Score`
  (params (ChangeInScore :type Integer))
  (bind _returnvalue (`IncrementGameScore.GetIncrementGameScore` ChangeInScore (`self.Score`)))
  (set `self.Score` _returnvalue))

(fn `UserConstructionScript`)